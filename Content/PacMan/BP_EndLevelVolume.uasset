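; BP_EndLevelVolume is an end-of-level trigger volume for the Pac-Man game.
; On BeginPlay it caches references to the GameManager and PacMan actors.
; When PacMan overlaps it, it calls the GameManager's WinEvent if LevelCompleted is set.
; Otherwise it teleports PacMan to TeleportPos by setting the root component's world location without sweeping.
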(event Collision|EventActorBeginOverlap
  (params (OtherActor :type Actor%20Object%20Reference))
  (bind _gm_ref (Variables|Default|GetGM_Ref))
  (if (== (Utilities|GetClass OtherActor) "/Game/PacMan/PacMan.PacMan_C")
    (if (Variables|/Game/PacMan/GameManager.GameManager_C|GetLevelCompleted _gm_ref)
      (Default|WinEvent _gm_ref)
      (else
        (Transformation|SetWorldLocation (Variables|/Script/Engine.Actor|GetRootComponent (Variables|Default|GetPG_Ref)) (Variables|Default|GetTeleportPos) false false)))))

(event EventBeginPlay
  (bind _returnvalue (Actor|GetActorOfClass "/Game/PacMan/GameManager.GameManager_C"))
  (Variables|Default|SetGM_Ref _returnvalue)
  (bind _returnvalue_2 (Actor|GetActorOfClass "/Game/PacMan/PacMan.PacMan_C"))
  (Variables|Default|SetPG_Ref _returnvalue_2))

(fn ConstructionScript)